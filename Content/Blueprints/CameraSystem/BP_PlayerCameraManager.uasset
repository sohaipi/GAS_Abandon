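; Player camera manager that drives an ALS-style first/third-person camera for targets tagged "M9", deferring to default behavior otherwise.
; OnPossess links the pawn and controller to the camera AnimBP, whose curves supply lag, offset and blend values.
; Each update reads pawn interface data, smooths rotation and yaw-relative per-axis pivot lag, then applies offsets.
; A sphere trace corrects obstructed positions before first-person and debug-view blending.
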(event Custom|OnPossess
  (params (New%20Pawn :type Pawn%20Object%20Reference))
  ;[1 1 1] 有角色更新时，需要刷新镜头控制，在角色控制器中调用
  (Variables|Default|SetControlledPawn New%20Pawn)
  (bind _asanim_bp_player_camera_behavior (Utilities|Casting|CastToAnimBP_PlayerCameraBehavior (Components|SkeletalMesh|GetAnimInstance (Variables|Default|GetCameraBehavior))))
  (Variables|/Game/Blueprints/CameraSystem/AnimBP_PlayerCameraBehavior.AnimBP_PlayerCameraBehavior_C|SetControlledPawn _asanim_bp_player_camera_behavior (Variables|Default|GetControlledPawn))
  (Variables|/Game/Blueprints/CameraSystem/AnimBP_PlayerCameraBehavior.AnimBP_PlayerCameraBehavior_C|SetPlayerController _asanim_bp_player_camera_behavior (Game|Player|GetOwningPlayerController)))

(fn ConstructionScript)

(fn BlueprintUpdateCamera
  (params (CameraTarget :type Actor%20Object%20Reference))
  (if (Actor|ActorHasTag CameraTarget "M9")
    (bind (_location _rotation _fov) (CallFunction|CustomCameraBehavior))
    (return _location _rotation _fov true)
    (else
      (bind (_newcameralocation _newcamerarotation _newcamerafov _returnvalue) (|CallParentFunction CameraTarget))
      (return _newcameralocation _newcamerarotation _newcamerafov _returnvalue))))

(fn CustomCameraBehavior
  (Utilities|FlowControl|Sequence
    (:then_0
      ;[1 1 1] NO1 通过相机接口从角色蓝图中拿到角色相机相关参数，以实现对人物移动时的相机追踪
      (bind _returnvalue (Class|BPICameraSystem|BPIGetTPPivotTarget(Message) (Variables|Default|GetControlledPawn)))
      (LocalVariables|SetPivot%20Target _returnvalue)
      (bind _returnvalue_2 (Class|BPICameraSystem|BPIGetFPCameraTarget(Message) (Variables|Default|GetControlledPawn)))
      (LocalVariables|SetFP%20Target _returnvalue_2)
      (bind (_rightshoulder _tp_fov _fp_fov) (Class|BPICameraSystem|BPIGetCameraParameters(Message) (Variables|Default|GetControlledPawn)))
      (LocalVariables|SetTP%20Fov _tp_fov)
      (LocalVariables|SetFP%20Fov _fp_fov))
    (:then_1
      ;[1 1 1] NO2 获取控制器旋转并对其插值，使相机归位更平滑
      (Variables|Default|SetTargetCameraRotation (Math|Rotator|Lerp(Rotator) (Math|Interpolation|RInterpTo (Camera|GetCameraRotation) (Transformation|GetActorRotation (Game|Player|GetOwningPlayerController)) (Utilities|Time|GetWorldDeltaSeconds) (CallFunction|GetCameraBehaviorParam "RotationLagSpeed")) (Variables|Default|GetDebug%20View%20Rotation) (CallFunction|GetCameraBehaviorParam "Override_Debug") true)))
    (:then_2
      ;[1 1 1] NO3 处理人物移动带来的平滑问题，以pivot点为终点，拆分三个轴的滞后平滑表现
      (Variables|Default|SetSmoothed%20Pivot%20Target (Math|Transform|MakeTransform (CallFunction|CaculateAxisIndependentLag (.location (Variables|Default|GetSmoothed%20Pivot%20Target)) (.location (LocalVariables|GetPivot%20Target)) (Variables|Default|GetTargetCameraRotation) (Math|Vector|MakeVector (CallFunction|GetCameraBehaviorParam "PivotLagSpeed_X") (CallFunction|GetCameraBehaviorParam "PivotLagSpeed_Y") (CallFunction|GetCameraBehaviorParam "PivotLagSpeed_Z"))) (.rotation (LocalVariables|GetPivot%20Target)))))
    (:then_3
      ;[1 1 1] NO4 用追踪锚点的旋转提取方向向量并做缩放，将锚点向指定方向做偏移 作为最终锚点
      (Variables|Default|SetPivotLocation (+ (.location (Variables|Default|GetSmoothed%20Pivot%20Target)) (* (Math|Vector|GetForwardVector (.rotation (Variables|Default|GetSmoothed%20Pivot%20Target))) (CallFunction|GetCameraBehaviorParam "PivotOffset_X")) (* (Math|Vector|GetUpVector (.rotation (Variables|Default|GetSmoothed%20Pivot%20Target))) (CallFunction|GetCameraBehaviorParam "PivotOffset_Z")) (* (Math|Vector|GetRightVector (.rotation (Variables|Default|GetSmoothed%20Pivot%20Target))) (CallFunction|GetCameraBehaviorParam "PivotOffset_Y")))))
    (:then_4
      ;[1 1 1] NO5 以最终点添加上正确的镜头偏移参数
      (Variables|Default|SetTargetCameraLocation (Math|Vector|Lerp(Vector) (+ (Variables|Default|GetPivotLocation) (* (Math|Vector|GetForwardVector (Variables|Default|GetTargetCameraRotation)) (Variables|Default|GetNewVar_0)) (* (Math|Vector|GetUpVector (Variables|Default|GetTargetCameraRotation)) (CallFunction|GetCameraBehaviorParam "CameraOffset_Z")) (* (Math|Vector|GetRightVector (Variables|Default|GetTargetCameraRotation)) (CallFunction|GetCameraBehaviorParam "CameraOffset_Y"))) (+ (.location (LocalVariables|GetPivot%20Target)) (Variables|Default|GetDebugView%20Offset)) (CallFunction|GetCameraBehaviorParam "Override_Debug"))))
    (:then_5
      ;[1 1 1] NO6 碰撞检测避障
      (bind (_traceorigin _traceradius _tracechannel) (Class|BPICameraSystem|BPIGetTPTraceParams(Message) (Variables|Default|GetControlledPawn)))
      (bind _outhit (Collision|SphereTraceByChannel _traceorigin (Variables|Default|GetTargetCameraLocation) _traceradius _tracechannel false 0 (CallFunction|GetDebugTraceType "None")))
      (if (and (.bBlockingHit (Collision|BreakHitResult _outhit)) (not (.bInitialOverlap (Collision|BreakHitResult _outhit))))
        (Variables|Default|SetTargetCameraLocation (+ (- (.Location (Collision|BreakHitResult _outhit)) (.TraceEnd (Collision|BreakHitResult _outhit))) (Variables|Default|GetTargetCameraLocation)))))
    (:then_6
      ;[1 1 1] NO7 绘制表现
      (Class|BPIController|BP|GetDebugInfo(Message) (Game|Player|GetOwningPlayerController))
      (if false
        (Rendering|Debug|DrawDebugSphere (.location (LocalVariables|GetPivot%20Target)) 15.0 6 "(R=0.962500,G=0.022360,B=0.004011,A=1.000000)" 0.0 1.0)
        (Rendering|Debug|DrawDebugSphere (.location (Variables|Default|GetSmoothed%20Pivot%20Target)) 15.0 6 "(R=0.207796,G=0.025000,B=1.000000,A=1.000000)" 0.0 1.0)
        (Rendering|Debug|DrawDebugSphere (Variables|Default|GetPivotLocation) 15.0 6 "(R=0.007638,G=0.032307,B=0.170833,A=1.000000)" 0.0 1.0)
        (Rendering|Debug|DrawDebugLine (.location (LocalVariables|GetPivot%20Target)) (.location (Variables|Default|GetSmoothed%20Pivot%20Target)) "(R=0.680208,G=0.000000,B=0.055117,A=1.000000)" 0.0 2.0)
        (Rendering|Debug|DrawDebugLine (.location (Variables|Default|GetSmoothed%20Pivot%20Target)) (Variables|Default|GetPivotLocation) "(R=0.000000,G=0.017803,B=0.971875,A=1.000000)" 0.0 2.0)))
    (:then_7
      ;[1 1 1] NOE 根据第一、三视角权重输出最终参数
      (return (.Location (Math|Transform|BreakTransform (Math|Transform|Lerp(Transform) (Math|Transform|Lerp(Transform) (Math|Transform|MakeTransform (Variables|Default|GetTargetCameraLocation) (Variables|Default|GetTargetCameraRotation)) (Math|Transform|MakeTransform (LocalVariables|GetFP%20Target) (Variables|Default|GetTargetCameraRotation)) (CallFunction|GetCameraBehaviorParam "Weight_FirstPerson")) (Math|Transform|MakeTransform (Variables|Default|GetTargetCameraLocation) (Variables|Default|GetDebug%20View%20Rotation)) (CallFunction|GetCameraBehaviorParam "Override_Debug")))) (.Rotation (Math|Transform|BreakTransform (Math|Transform|Lerp(Transform) (Math|Transform|Lerp(Transform) (Math|Transform|MakeTransform (Variables|Default|GetTargetCameraLocation) (Variables|Default|GetTargetCameraRotation)) (Math|Transform|MakeTransform (LocalVariables|GetFP%20Target) (Variables|Default|GetTargetCameraRotation)) (CallFunction|GetCameraBehaviorParam "Weight_FirstPerson")) (Math|Transform|MakeTransform (Variables|Default|GetTargetCameraLocation) (Variables|Default|GetDebug%20View%20Rotation)) (CallFunction|GetCameraBehaviorParam "Override_Debug")))) (Math|Float|Lerp (LocalVariables|GetTP%20Fov) (LocalVariables|GetFP%20Fov) (CallFunction|GetCameraBehaviorParam "Weight_FirstPerson"))))))

(fn GetCameraBehaviorParam
  (params (Curve%20Name :type Name))
  (bind _camerabehavior (Variables|Default|GetCameraBehavior))
  (bind _returnvalue (Components|SkeletalMesh|GetAnimInstance _camerabehavior))
  ;[1 1 1] 传送相机动画实例中的浮点曲线值
  (Utilities|IsValid _returnvalue
    (:Is%20Valid
      (return (Animation|Curves|GetCurveValue _returnvalue Curve%20Name)))
    (:Is%20Not%20Valid
      (return 0.0))))

(fn CaculateAxisIndependentLag
  (params (Current%20Location :type Vector) (Target%20Locaiton :type Vector) (Camera%20Rotation :type Rotator) (Lag%20Speeds :type Vector))
  (bind _returnvalue (Utilities|Time|GetWorldDeltaSeconds))
  ;[1 1 1] 以第二步的同一旋转体Yaw逆旋转为空间坐标；并在三个轴做差速平滑；使用Yaw值转回世界坐标
  (LocalVariables|SetCamera%20Rotation%20Yaw (Math|Rotator|MakeRotator 0.0 0.0 (.yaw Camera%20Rotation)))
  (return (Math|Vector|RotateVector (Math|Vector|MakeVector (Math|Interpolation|FInterpTo (.x (Math|Vector|UnrotateVector Current%20Location (LocalVariables|GetCamera%20Rotation%20Yaw))) (.x (Math|Vector|UnrotateVector Target%20Locaiton (LocalVariables|GetCamera%20Rotation%20Yaw))) _returnvalue (.x Lag%20Speeds)) (Math|Interpolation|FInterpTo (.y (Math|Vector|UnrotateVector Current%20Location (LocalVariables|GetCamera%20Rotation%20Yaw))) (.y (Math|Vector|UnrotateVector Target%20Locaiton (LocalVariables|GetCamera%20Rotation%20Yaw))) _returnvalue (.y Lag%20Speeds)) (Math|Interpolation|FInterpTo (.z (Math|Vector|UnrotateVector Current%20Location (LocalVariables|GetCamera%20Rotation%20Yaw))) (.z (Math|Vector|UnrotateVector Target%20Locaiton (LocalVariables|GetCamera%20Rotation%20Yaw))) _returnvalue (.z Lag%20Speeds))) (LocalVariables|GetCamera%20Rotation%20Yaw))))

(fn GetDebugTraceType
  (params (ShowTraceType :type EDrawDebugTrace%20Enum :default "None"))
  (Class|BPIController|BP|GetDebugInfo(Message) (Game|Player|GetOwningPlayerController))
  (if true
    (return ShowTraceType)
    (else
      (return "None"))))