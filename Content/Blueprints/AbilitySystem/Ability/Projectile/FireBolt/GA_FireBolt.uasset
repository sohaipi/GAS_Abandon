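; GA_FireBolt is a gameplay ability that fires a projectile, by its name a fire bolt, at the location under the mouse cursor.
; It gets the hit location from mouse target data and sets it as the avatar's warping target through CombatInterface.
; It then plays the AM_FireBolt montage, waits for the Event.Montage.Fire gameplay event to spawn the projectile toward that location, and ends after a short delay.
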(event Ability|EventActivateAbility
  (bind _data (|CreatTargetDataUnderMouse)
    (:then
      (bind _output_get (Variables|Default|SetTargetLocation (.Location (Collision|BreakHitResult (Ability|TargetData|GetHitResultfromTargetData _data)))))
      (bind _ascombat_interface (Utilities|Casting|CastToCombatInterface (Ability|GetAvatarActorfromActorInfo)))
      (Class|CombatInterface|UpdateWarpingTarget _ascombat_interface _output_get)
      (|PlayMontageandWaitProxy "None" "/Game/Blueprints/AbilitySystem/Ability/AM_FireBolt.AM_FireBolt" 1.0 "None" true 1.0 0.0 false
        (:then
          (Ability|Tasks|WaitGameplayEvent "(TagName=\"Event.Montage.Fire\")" 0
            (:EventReceived
              (Class|B9ProjectileSpell|SpawnProjectile (Variables|Default|GetTargetLocation))
              (Utilities|FlowControl|Delay 0.5)
              (Ability|EndAbility))))))))