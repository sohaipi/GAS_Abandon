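; Enemy ranged attack ability that fires a projectile at the avatar's combat target, timed to an attack montage.
; On activation it sets the warping target to the combat target's location, then plays a montage from the avatar's tagged attack montages.
; A gameplay event matching the stored montage tag spawns the projectile and ends the ability.
; Montage, tag and weapon socket come from separate random-pick calls, so they can differ.
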(event Ability|EventActivateAbility
  (bind _returnvalue (Ability|GetAvatarActorfromActorInfo))
  (bind _returnvalue_2 (Class|CombatInterface|GetCombatTarget(Message) _returnvalue))
  (bind _ascombat_interface (Utilities|Casting|CastToCombatInterface _returnvalue))
  (Class|CombatInterface|UpdateWarpingTarget _ascombat_interface (Transformation|GetActorLocation _returnvalue_2))
  (bind _returnvalue_3 (Class|CombatInterface|GetAttackMontages _ascombat_interface))
  (bind _output_get (Variables|Default|SetMontage%20Tag (.MontageTag (Utilities|Struct|BreakTaggedMontage (Class|B9DamageGameplayAbility|GetRandomTaggedMontagefromArray _returnvalue_3)))))
  (|PlayMontageandWaitProxy "None" (.Montage (Utilities|Struct|BreakTaggedMontage (Class|B9DamageGameplayAbility|GetRandomTaggedMontagefromArray _returnvalue_3))) 1.0 "None" false 1.0 0.0 false
    (:then
      (Ability|Tasks|WaitGameplayEvent _output_get 0
        (:EventReceived
          (Class|CombatInterface|GetCombatTipLocation(Message) (Ability|GetAvatarActorfromActorInfo) _output_get)
          (bind _returnvalue_4 (Class|CombatInterface|GetCombatTarget(Message) (Ability|GetAvatarActorfromActorInfo)))
          (Class|B9ProjectileSpell|SpawnProjectile (Transformation|GetActorLocation _returnvalue_4) (.WeaponSocketTag (Utilities|Struct|BreakTaggedMontage (Class|B9DamageGameplayAbility|GetRandomTaggedMontagefromArray _returnvalue_3))))
          (Ability|EndAbility))))
    (:OnCompleted
      (Ability|EndAbility :!label _label))
    (:OnInterrupted
      (goto _label))
    (:OnCancelled
      (goto _label))))