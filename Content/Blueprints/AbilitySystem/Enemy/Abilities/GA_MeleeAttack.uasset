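; Enemy melee attack ability that warps toward the combat target, plays a random attack montage and damages nearby players.
; The montage's tag event triggers a small sphere query at the tagged weapon socket, drawn as a debug sphere.
; Non-friendly live players found take damage, and any hit fires a melee impact GameplayCue carrying the montage tag.
; The ability ends after that check or when the montage finishes or is interrupted.
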(event Ability|EventActivateAbility
  (bind _returnvalue (Ability|GetAvatarActorfromActorInfo))
  (bind _returnvalue_2 (Ability|GetAvatarActorfromActorInfo))
  (Variables|Default|SetbHasHitTarget false)
  (bind _returnvalue_3 (Class|CombatInterface|GetCombatTarget(Message) _returnvalue_2))
  (bind _ascombat_interface (Utilities|Casting|CastToCombatInterface _returnvalue_2))
  (Class|CombatInterface|UpdateWarpingTarget _ascombat_interface (Transformation|GetActorLocation _returnvalue_3))
  (bind _returnvalue_4 (Class|CombatInterface|GetAttackMontages _ascombat_interface))
  (bind _output_get (Variables|Default|SetTaggedMontage (Class|B9DamageGameplayAbility|GetRandomTaggedMontagefromArray _returnvalue_4)))
  (|PlayMontageandWaitProxy "None" (.Montage (Utilities|Struct|BreakTaggedMontage _output_get)) 1.0 "None" false 1.0 0.0 false
    (:then
      (Ability|Tasks|WaitGameplayEvent (.montagetag (Variables|Default|GetTaggedMontage)) 0
        (:EventReceived
          (bind _returnvalue_5 (Class|CombatInterface|GetCombatTipLocation(Message) _returnvalue (.weaponsockettag (Variables|Default|GetTaggedMontage))))
          (bind _outoverlappingactors (Class|B9ASCBlueprintLibrary|GetLivePlayersWithinRadius _returnvalue (Utilities|Array|MakeArray _returnvalue) 45.0 _returnvalue_5))
          (Rendering|Debug|DrawDebugSphere _returnvalue_5 45.0 12 "(R=0.016101,G=0.000000,B=1.000000,A=1.000000)" 1.0 2.0)
          (for _array_element _outoverlappingactors
            (bind _returnvalue_6 (Class|B9ASCBlueprintLibrary|IsNotFriends (Ability|GetAvatarActorfromActorInfo) _array_element))
            (if _returnvalue_6
              (Variables|Default|SetbHasHitTarget true)
              (Class|B9DamageGameplayAbility|CauseDamage _array_element)))
          (if (Variables|Default|GetbHasHitTarget)
            (Class|GameplayAbility|ExecuteGameplayCuewithParams "(TagName=\"GameplayCue.MeleeImpact\")" (Ability|GameplayCue|MakeGameplayCueParameters :AggregatedSourceTags (GameplayTags|MakeGameplayTagContainerfromTag (.MontageTag (Utilities|Struct|BreakTaggedMontage (Variables|Default|GetTaggedMontage)))) :Location _returnvalue_5 :EffectCauser (Ability|GetAvatarActorfromActorInfo) :SourceObject _array_element)))
          (Ability|EndAbility))))
    (:OnCompleted
      (Ability|EndAbility :!label _label))
    (:OnInterrupted
      (goto _label))
    (:OnCancelled
      (goto _label))))