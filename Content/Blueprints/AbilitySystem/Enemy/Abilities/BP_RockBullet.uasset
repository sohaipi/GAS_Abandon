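; BP_RockBullet is a rock projectile for enemy abilities that tumbles visually using a slingshot rock mesh.
; BeginPlay picks random yaw, pitch and roll rates, each able to spin in either direction.
; Tick applies those rates, scaled by delta time, as local rotation on the mesh component.
; The graphs here contain no movement, collision or damage logic.
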(event EventBeginPlay
  (bind _returnvalue (Math|Random|RandomFloatinRange -5e+02 5e+02))
  (Variables|Default|SetYawRoRate _returnvalue)
  (Variables|Default|SetPitchRoRate _returnvalue)
  (Variables|Default|SetRollRoRate _returnvalue))

(event Collision|EventActorBeginOverlap
  (params (OtherActor :type Actor%20Object%20Reference)))

(event EventTick
  (params (DeltaSeconds :type Float%20%28single-precision%29))
  (Transformation|AddLocalRotation (Variables|Default|GetSM_SlingshotRock) (Math|Rotator|MakeRotator (* DeltaSeconds (Variables|Default|GetRollRoRate)) (* DeltaSeconds (Variables|Default|GetPitchRoRate)) (* DeltaSeconds (Variables|Default|GetYawRoRate))) false false))

(fn ConstructionScript)