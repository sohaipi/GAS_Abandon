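; M9 playable-style character Blueprint that extends a parent locomotion character with camera targets, roll and mantle assets, and held-object visuals.
; Camera interface functions supply the head-root midpoint pivot, shoulder-based trace origin and first-person socket.
; Overlay changes refresh the held object, attaching an M4A1 to a virtual hand bone for Rifle and clearing it for other states.
; High and falling-catch mantles hide the object until the mantle ends.
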(event EventBeginPlay)

(event Collision|EventActorBeginOverlap
  (params (OtherActor :type Actor%20Object%20Reference)))

(event EventTick
  (params (DeltaSeconds :type Float%20%28single-precision%29))
  (|CallParentFunction DeltaSeconds))

(fn ConstructionScript
  (|CallParentFunction))

(fn BPIGetTPTraceParams
  (bind _mesh (Variables|Character|GetMesh))
  (if (Variables|Default|GetRightShoulder)
    (return (Transformation|GetSocketLocation _mesh "TP_CameraTrace_R") 8.0 "TraceTypeQuery1")
    (else
      (return (Transformation|GetSocketLocation _mesh "TP_CameraTrace_L") 8.0 "TraceTypeQuery1"))))

(fn BPIGetTPPivotTarget
  (bind _mesh (Variables|Character|GetMesh))
  ;[1 1 1] 头脚相机获取角色腰部位置为摄像机的基础锚点
  (return (Math|Transform|MakeTransform (Math|Vector|GetVectorArrayAverage (Utilities|Array|MakeArray (Transformation|GetSocketLocation _mesh "head") (Transformation|GetSocketLocation _mesh "root"))) (Transformation|GetActorRotation))))

(fn BPIGetFPCameraTarget
  (return (Transformation|GetSocketLocation (Variables|Character|GetMesh) "FP_Camera")))

(fn GetRollAnimation
  (return (Variables|Default|GetLandRoll%20Default)))

(fn GetMantleAsset
  (params (MantleType :type M9_MantleType%20Enum :default "NewEnumerator0"))
  (switch Utilities|FlowControl|Switch|SwitchonM9_MantleType MantleType
    (:NewEnumerator0
      _)
    (:NewEnumerator1
      (return (Variables|Default|GetMantle1mDefault)))
    (:NewEnumerator2
      _))
  (return (Variables|Default|GetMantle2mDefault)))

(fn UpdateHeldObject
  (switch Utilities|FlowControl|Switch|SwitchonM9_OverlayState (Variables|Default|GetOverlay%20State)
    (:NewEnumerator0
      (HeldObject|ClearObject :!label _label))
    (:NewEnumerator1
      (goto _label))
    (:NewEnumerator2
      (goto _label))
    (:NewEnumerator3
      (goto _label))
    (:NewEnumerator4
      (goto _label))
    (:NewEnumerator14
      (HeldObject|AttachtoHand 0 "/Game/Resource/AdvancedLocomotionV4/Props/Meshes/M4A1.M4A1" 0 false "0, 0, 0"))))

(fn ClearObject
  (bind _skeletalmesh (Variables|Default|GetSkeletalMesh))
  (Components|StaticMesh|SetStaticMesh (Variables|Default|GetStaticMesh) 0)
  (Components|SkinnedMesh|SetSkinnedAssetandUpdate _skeletalmesh 0 true)
  (Class|SkeletalMeshComponent|SetAnimClass _skeletalmesh))

(fn AttachtoHand
  (params (NewStaticMesh :type Static%20Mesh%20Object%20Reference) (NewSkeletalMesh :type Skeletal%20Mesh%20Object%20Reference) (NewAnimClass :type Object%20Class%20Reference) (LeftHand :type Boolean) (Offset :type Vector))
  (Utilities|FlowControl|Sequence
    (:then_0
      (HeldObject|ClearObject))
    (:then_1
      (bind _newstaticmesh (LocalVariables|GetNewStaticMesh)
        (:then
          (Components|StaticMesh|SetStaticMesh (Variables|Default|GetStaticMesh) _newstaticmesh))
        (:else)))
    (:then_2
      (bind _newskeletalmesh (LocalVariables|GetNewSkeletalMesh)
        (:then
          (Components|SkinnedMesh|SetSkinnedAssetandUpdate (Variables|Default|GetSkeletalMesh) _newskeletalmesh true)
          (LocalVariables|GetNewAnimClass
            (:then
              (Class|SkeletalMeshComponent|SetAnimClass (Variables|Default|GetSkeletalMesh)))
            (:else)))
        (:else)))
    (:then_3
      (Transformation|AttachComponentToComponent (Variables|Default|GetHeld%20Object) (Variables|Character|GetMesh) (select LeftHand "VB LHS_ik_hand_gun" "VB RHS_ik_hand_gun") "SnapToTarget" "SnapToTarget" "SnapToTarget" true)
      (Transformation|SetRelativeLocation (Variables|Default|GetHeld%20Object) Offset false false))))

(fn UpdateHeldObjectAnimations)

(fn OnOverlayStateChanged
  (params (NewOverlayState :type M9_OverlayState%20Enum :default "NewEnumerator0"))
  (|CallParentFunction NewOverlayState)
  (HeldObject|UpdateHeldObject))

(fn MantleStart
  (params (MantleHeight :type Float%20%28double-precision%29) (MantleLedgeWS :type M9%20Component%20and%20Transform%20Structure) (MantleType :type M9_MantleType%20Enum :default "NewEnumerator0"))
  (|CallParentFunction MantleHeight MantleLedgeWS MantleType)
  (switch Utilities|FlowControl|Switch|SwitchonM9_MantleType MantleType
    (:NewEnumerator0
      _)
    (:NewEnumerator2
      _))
  (HeldObject|ClearObject))

(fn MantleEnd
  (|CallParentFunction)
  (HeldObject|UpdateHeldObject))