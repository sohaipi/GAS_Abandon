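; BP_LineBox is a moving object actor whose static mesh travels back and forth along a spline.
; While movement is enabled, Tick advances a clamped time in the current direction, then at either end pauses for a wait time and reverses.
; UpdateObjectLocation remaps that time through a float curve to shape the motion along the spline.
; The construction script sets the spline duration and previews the configurable start position.
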(event EventBeginPlay)

(event Collision|EventActorBeginOverlap
  (params (OtherActor :type Actor%20Object%20Reference)))

(event EventTick
  (params (DeltaSeconds :type Float%20%28single-precision%29))
  (Variables|Default|SetDelta%20Seconds DeltaSeconds)
  (if (Variables|Default|GetCanMove)
    (Variables|Default|SetMovementTime (Math|Float|Clamp(Float) (+ (Variables|Default|GetMovementTime) (* (Variables|Default|GetMovementDirection) (Variables|Default|GetDelta%20Seconds))) 0.0 (Variables|/Script/Engine.SplineComponent|GetDuration (Variables|Default|GetSpline))))
    (Math|Integer|CompareInt (Variables|Default|GetMovementDirection)
      (:>
        (if (Math|Float|NearlyEqual(Float) (Variables|/Script/Engine.SplineComponent|GetDuration (Variables|Default|GetSpline)) (Variables|Default|GetMovementTime) 1e-06)
          (Variables|Default|SetCanMove false :!label _label)
          (Variables|Default|SetMovementDirection (* (Variables|Default|GetMovementDirection) -1))
          (Utilities|FlowControl|Delay (Variables|Default|GetWaitTime))
          (Variables|Default|SetCanMove true)
          (else
            (CallFunction|UpdateObjectLocation :!label _label_2))))
      (:<
        (if (Math|Float|NearlyEqual(Float) (Variables|Default|GetMovementTime) 0.0 1e-06)
          (goto _label)
          (else
            (goto _label_2)))))))

(fn ConstructionScript
  (|CallParentFunction)
  (Variables|/Script/Engine.SplineComponent|SetDuration (Variables|Default|GetSpline) (Variables|Default|GetDuration))
  (Variables|Default|SetMovementTime (* (Variables|Default|GetDuration) (Variables|Default|GetStartPosition)))
  (CallFunction|UpdateObjectLocation))

(fn UpdateObjectLocation
  (bind _spline (Variables|Default|GetSpline))
  (bind _duration (Variables|/Script/Engine.SplineComponent|GetDuration _spline))
  (Transformation|SetWorldLocation (Variables|Default|GetStaticMesh) (Spline|GetLocationatTime (Variables|Default|GetSpline) (Math|Float|MapRangeClamped (Math|Curves|GetFloatValue (Variables|Default|GetMovementCurrve) (Math|Float|NormalizetoRange (Variables|Default|GetMovementTime) 0.0 _duration)) 0.0 1.0 0.0 _duration) "World" false) false false))