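; Player controller for the character that forwards possession to the custom camera manager and hosts the HUD, overlay-state switcher and debug toggles.
; Holding the overlay input opens a switcher widget in slowed time, cycle inputs step through states, and release applies the selection.
; Debug keys toggle HUD, slow motion and character info flags.
; A getter exposes debug state, suppressing character info while the overlay menu is open.
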(event EventBeginPlay
  ;[1 1 1] 注释
  (bind _returnvalue (UserInterface|CreateWidget "/Game/Blueprints/UI/M9_HUD.M9_HUD_C" self))
  (bind _output_get (Variables|Default|SetM9_HUD _returnvalue))
  (UserInterface|Viewport|AddtoViewport _output_get 0)
  ;[1 0.7528 0.3881] 可拓展查看其它角色
  (Variables|调试|SetDebugFocusCharacter (Game|GetPlayerCharacter 0)))

(event EventPossess
  (params (PossessedPawn :type Pawn%20Object%20Reference))
  ;[1 1 1] 操控角色时，刷新摄像机控制器的角色，与相机管理器通信
  (bind _asbp_player_camera_manager (Utilities|Casting|CastToBP_PlayerCameraManager (Variables|Default|GetPlayerCameraManager)))
  (Default|OnPossess _asbp_player_camera_manager PossessedPawn))

(event Input|ActionEvents|InputActionOpenOverlayMenu
  (params (Key :type Key%20Structure :default "None"))
  ;[1 1 1] 状态轮盘
  (:Pressed
    (Variables|Default|SetOverlayMenuOpen true)
    (if (Variables|调试|GetSlomo)
      _
      (else
        (Utilities|Time|SetGlobalTimeDilation 0.3)))
    (bind _returnvalue (UserInterface|CreateWidget "/Game/Blueprints/UI/OverlayStateSwitcher.OverlayStateSwitcher_C" self))
    (bind _output_get (Variables|Default|SetOverlaySwticher _returnvalue))
    (UserInterface|Viewport|AddtoViewport _output_get 0)
    (Audio|PlaySound2D "/Game/Resource/AdvancedLocomotionV4/Audio/UI/Click.Click" 1.0 1.0 0.0 0 0))
  (:Released
    (Variables|Default|SetOverlayMenuOpen false)
    (if (Variables|调试|GetSlomo)
      _
      (else
        (Utilities|Time|SetGlobalTimeDilation 1.0)))
    (Default|SelectOverlayState (Variables|Default|GetOverlaySwticher))
    (Widget|RemovefromParent (Variables|Default|GetOverlaySwticher))
    (Audio|PlaySound2D "/Game/Resource/AdvancedLocomotionV4/Audio/UI/Click.Click" 1.0 1.0 0.0 0 0)))

(event Input|ActionEvents|InputActionCycleOverlayUp
  (params (Key :type Key%20Structure :default "None"))
  ;[1 1 1] 状态轮盘
  (:Pressed
    (if (Variables|Default|GetOverlayMenuOpen)
      (bind _overlayswticher (Variables|Default|GetOverlaySwticher)
        (:then
          (Default|CycleState _overlayswticher true)
          (Audio|PlaySound2D "/Game/Resource/AdvancedLocomotionV4/Audio/UI/Click.Click" 1.0 1.0 0.0 0 0))
        (:else)))))

(event Input|ActionEvents|InputActionCycleOverlayDown
  (params (Key :type Key%20Structure :default "None"))
  ;[1 1 1] 状态轮盘
  (:Pressed
    (if (Variables|Default|GetOverlayMenuOpen)
      (bind _overlayswticher (Variables|Default|GetOverlaySwticher)
        (:then
          (Default|CycleState _overlayswticher false)
          (Audio|PlaySound2D "/Game/Resource/AdvancedLocomotionV4/Audio/UI/Click.Click" 1.0 1.0 0.0 0 0))
        (:else)))))

(event Input|KeyboardEvents|Tab
  (params (Key :type Key%20Structure :default "None"))
  ;[1 1 1] Debug
  (:Pressed
    (Variables|调试|SetShowHUD (not (Variables|调试|GetShowHUD)))))

(event Input|KeyboardEvents|I
  (params (Key :type Key%20Structure :default "None"))
  ;[1 1 1] Debug
  (:Pressed
    (Variables|调试|SetShowCharacterInfo (not (Variables|调试|GetShowCharacterInfo)))))

(event Input|KeyboardEvents|Z
  (params (Key :type Key%20Structure :default "None"))
  ;[1 1 1] Debug
  (:Pressed
    (bind _output_get (Variables|调试|SetSlomo (not (Variables|调试|GetSlomo))))
    (if _output_get
      (Utilities|Time|SetGlobalTimeDilation 0.1)
      (else
        (Utilities|Time|SetGlobalTimeDilation 1.0)))))

(fn ConstructionScript)

(fn BP|GetDebugInfo
  (return (Variables|调试|GetDebugFocusCharacter) (Variables|调试|GetDebugView) (Variables|调试|GetShowHUD) (Variables|调试|GetShowTraces) (Variables|调试|GetShowDebugShapes) (Variables|调试|GetShowLayerColors) (Variables|调试|GetSlomo) (and (Variables|调试|GetShowCharacterInfo) (not (Variables|Default|GetOverlayMenuOpen)))))