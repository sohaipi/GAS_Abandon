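; CalculateRotationAmount is an animation modifier that bakes a turning curve into an animation sequence.
; On apply, it recreates the named float curve, removing any existing one first.
; It keys each frame with the root bone's yaw difference to the adjacent frame in playback direction, scaled by the absolute rate scale.
; A negative rate scale selects the previous frame instead of the next, accounting for reversed playback.
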(event EventOnApply
  (params (AnimationSequence :type Anim%20Sequence%20Object%20Reference))
  (bind _rootbonename (Variables|Default|GetRootBoneName))
  ;[1 1 1] 生成动画的转向曲线
  (bind _output_get (Variables|Default|SetAnimSequence AnimationSequence))
  (bind _returnvalue (Class|AnimationBlueprintLibrary|DoesCurveExist _output_get (Variables|Default|GetCurveName) "RCT_Float"))
  (if _returnvalue
    (Class|AnimationBlueprintLibrary|RemoveCurve (Variables|Default|GetAnimSequence) (Variables|Default|GetCurveName) false))
  (Class|AnimationBlueprintLibrary|AddCurve (Variables|Default|GetAnimSequence) (Variables|Default|GetCurveName) "RCT_Float" false)
  (for _index (range 0 (Class|AnimationBlueprintLibrary|GetNumFrames (Variables|Default|GetAnimSequence)))
    (Class|AnimationBlueprintLibrary|AddFloatCurveKey (Variables|Default|GetAnimSequence) (Variables|Default|GetCurveName) (Class|AnimationBlueprintLibrary|GetTimeatFrame (Variables|Default|GetAnimSequence) _index) (* (- (.yaw (.rotation (Class|AnimationBlueprintLibrary|GetBonePoseforFrame (Variables|Default|GetAnimSequence) _rootbonename (+ _index (Math|Integer|SelectInt -1 1 (< (Class|AnimationBlueprintLibrary|GetRateScale (Variables|Default|GetAnimSequence)) 0.0))) false))) (.yaw (.rotation (Class|AnimationBlueprintLibrary|GetBonePoseforFrame (Variables|Default|GetAnimSequence) _rootbonename _index false)))) (Math|Float|Absolute(Float) (Class|AnimationBlueprintLibrary|GetRateScale (Variables|Default|GetAnimSequence)))))))