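; BP_FadeActor is a static mesh actor that can fade out and back in.
; Construction caches original materials and builds dynamic instances from separate fade materials.
; FadeOut swaps those in and plays a timeline driving their Fade parameter while keeping Visibility blocked; Fadein reverses it.
; On finish, a near-one value restores original materials, while a value at most half makes the mesh ignore the Visibility channel.
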(event EventFadeOut
  (CallFunction|SetMaterialstoDynamicInst)
  (bind _fade (Timeline|FadeTimeline Play)
    (:Update
      (for _array_element (Variables|Default|GetDynamicMaterialInstance)
        (Rendering|Material|SetScalarParameterValue _array_element "Fade" _fade :!class /Script/Engine.MaterialInstanceDynamic)
        (Collision|SetCollisionResponsetoChannel (Variables|Default|GetStaticMesh) "ECC_Visibility" "ECR_Block")))
    (:Finished
      (CallFunction|FadeFinish _fade))))

(event EventFadein
  (bind _fade (Timeline|FadeTimeline Reverse)
    (:Update
      (for _array_element (Variables|Default|GetDynamicMaterialInstance)
        (Rendering|Material|SetScalarParameterValue _array_element "Fade" _fade :!class /Script/Engine.MaterialInstanceDynamic)
        (Collision|SetCollisionResponsetoChannel (Variables|Default|GetStaticMesh) "ECC_Visibility" "ECR_Block")))
    (:Finished
      (CallFunction|FadeFinish _fade))))

(fn ConstructionScript
  (Utilities|Array|Clear (Variables|Default|GetDynamicMaterialInstance))
  (Variables|Default|SetOriginMaterial (Rendering|Material|GetMaterials (Variables|Default|GetStaticMesh)))
  (for _array_element (Variables|Default|GetFadeMaterialInstance)
    (bind _returnvalue (Rendering|Material|CreateDynamicMaterialInstance _array_element "None" "None" :!class /Script/Engine.KismetMaterialLibrary))
    (Utilities|Array|AddUnique (Variables|Default|GetDynamicMaterialInstance) _returnvalue)))

(fn SetMaterialstoDynamicInst
  (for (_array_element _array_index) (Variables|Default|GetDynamicMaterialInstance)
    (Rendering|Material|SetMaterial (Variables|Default|GetStaticMesh) _array_index _array_element)))

(fn ResetMaterials
  (for (_array_element _array_index) (Variables|Default|GetOriginMaterial)
    (Rendering|Material|SetMaterial (Variables|Default|GetStaticMesh) _array_index _array_element)))

(fn FadeFinish
  (params (FadePara :type Float%20%28single-precision%29))
  (if (>= FadePara 0.99)
    (CallFunction|ResetMaterials)
    (elif (<= FadePara 0.5)
      (Collision|SetCollisionResponsetoChannel (Variables|Default|GetStaticMesh) "ECC_Visibility" "ECR_Ignore"))))