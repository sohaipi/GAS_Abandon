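; BP_FlamePillar is an actor that gives its point light a continuous, randomly varied flame flicker.
; From BeginPlay, the FlameIntensity event randomly plays one of two timelines, each scaling DefaultIntensity by its curve value to set the light's intensity.
; When a timeline finishes, it calls FlameIntensity again, creating an endless loop without Tick.
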(event Custom|FlameIntensity
  (switch int (Math|Random|RandomIntegerinRange 0 1)
    (:Default
      (bind _flameintensity (Timeline|FlameIntensity_2 PlayFromStart)
        (:Update
          (Rendering|Components|Light|SetIntensity (Variables|Default|GetPointLight) (* _flameintensity (Variables|Default|GetDefaultIntensity))))
        (:Finished
          (CallFunction|FlameIntensity :!label _label))))
    (:0
      (bind _flameintensity_2 (Timeline|FlameIntensity_1 PlayFromStart)
        (:Update
          (Rendering|Components|Light|SetIntensity (Variables|Default|GetPointLight) (* _flameintensity_2 (Variables|Default|GetDefaultIntensity))))
        (:Finished
          (goto _label))))
    (:1
      (Timeline|FlameIntensity_2 PlayFromStart))))

(event EventBeginPlay
  (CallFunction|FlameIntensity))

(fn ConstructionScript)